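; BP_Spaceship is a scripted spaceship that plays a takeoff and drop sequence, then spawns an Astro actor.
; StartFlying sets door and drop flags on the skeletal mesh's anim Blueprint, fires particle effects, then hides the ship after a delay.
; It then calls StartDrop, which repositions and reveals the ship, plays the landing effect and spawns the Astro using arrow-component transforms.
; The construction script attaches the particle system to the mesh's "Agg" socket.
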(event Custom|StartFlying
  (bind _anim_bp (Variables|Default|GetAnim_BP))
  (Variables|/Game/main/spaceship_anime_blueprint.spaceship_anime_blueprint_C|Setb_door _anim_bp false)
  (Variables|/Game/main/spaceship_anime_blueprint.spaceship_anime_blueprint_C|Setb_drop _anim_bp true)
  (Components|Activation|Activate (Variables|Default|GetParticleSystem) true)
  (Utilities|FlowControl|Delay 4.0)
  (Rendering|SetActorHiddenInGame true)
  (CallFunction|StartDrop))

(event Custom|StartDrop
  (Transformation|SetActorTransform (Variables|Default|GetMake%20Transform) true true)
  (Rendering|SetActorHiddenInGame false)
  (Variables|/Game/main/spaceship_anime_blueprint.spaceship_anime_blueprint_C|Setb_drop (Variables|Default|GetAnim_BP) false)
  (Components|Activation|Activate (Variables|Default|GetLanding) true)
  (Utilities|FlowControl|Delay 6.0)
  (Game|SpawnActorfromClass "/Game/main/Astro.Astro_C" (Transformation|GetWorldTransform (Variables|Default|GetArrow)) "AlwaysSpawn" 0 (.Location (Math|Transform|BreakTransform (Transformation|GetWorldTransform (Variables|Default|GetArrow1)))) 0))

(event EventBeginPlay
  (bind _asspaceship_anime_blueprint (Utilities|Casting|CastTospaceship_anime_blueprint (Components|SkeletalMesh|GetAnimInstance (Variables|Default|GetSkeletalMesh))))
  (Variables|Default|SetAnim_BP _asspaceship_anime_blueprint))

(fn ConstructionScript
  (Transformation|AttachComponentToComponent (Variables|Default|GetParticleSystem) (Variables|Default|GetSkeletalMesh) "Agg" "SnapToTarget" "KeepRelative" "KeepRelative" true))